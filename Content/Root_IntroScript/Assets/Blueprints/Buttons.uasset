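; A shootable button that serves as one of two switches (A or B) for a linked BP_CircularGate.
; When a FirstPersonProjectile hits its Trigger, it plays a click sound once, at world origin.
; The hit also sets the gate's A or B flag according to IsA, turns the Sphere green and calls OpenDoor on the gate.
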(event `self.Trigger.OnComponentHit`
  (params (HitComponent :type "PrimitiveComponent Object Reference") (OtherActor :type "Actor Object Reference") (OtherComp :type "PrimitiveComponent Object Reference") (NormalImpulse :type "Vector Structure") (Hit :type "HitResult Structure (by ref)"))
  (bind _door (`self.Door`))
  (cast `/Game/Root_IntroScript/Core/Framework/FirstPersonProjectile` OtherActor)
  (`|ExecutionSequence`
    (:`then_0`
      (`/Engine/EditorBlueprintResources/StandardMacros.DoOnce` false
        (:`Completed`
          (`GameplayStatics.PlaySoundAtLocation` "/Game/Root_IntroScript/Assets/SFX/382574__josepharaoh99__sci-fi-two-part-click.382574__josepharaoh99__sci-fi-two-part-click" (0.0 0.0 0.0) (struct) 1.0 1.0 0.0 null null null))))
    (:`then_1`
      (bind _asbp_circular_gate (cast `/Game/Root_IntroScript/Assets/Blueprints/BP_CircularGate` (`self.Target`)))
      (set `self.Door` _asbp_circular_gate)
      (if (`self.bIsA`)
        (set `/Game/Root_IntroScript/Assets/Blueprints/BP_CircularGate.bAHasBeenHit` true _door)
        (else
          (set `/Game/Root_IntroScript/Assets/Blueprints/BP_CircularGate.bBHasBeenHit` true _door)))
      (`PrimitiveComponent.SetMaterial` (`self.Sphere`) 0 "/Game/Root_IntroScript/Assets/Materials/M_Color_Green_Inst.M_Color_Green_Inst")
      (`/Game/Root_IntroScript/Assets/Blueprints/BP_CircularGate.Open Door` (`self.Door`)))))

(fn `UserConstructionScript`)
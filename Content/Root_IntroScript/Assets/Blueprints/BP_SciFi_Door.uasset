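; BP_SciFi_Door is a sliding double door that opens when something enters its trigger and closes when it leaves.
; Trigger overlap begin and end play and reverse the Movement timeline, which lerps DoorL and DoorR between their start and end relative locations.
; The overlap events do not filter the actor or count occupants, so any end overlap starts the doors closing.
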(event `self.Trigger.OnComponentBeginOverlap`
  (params (OverlappedComponent :type "PrimitiveComponent Object Reference") (OtherActor :type "Actor Object Reference") (OtherComp :type "PrimitiveComponent Object Reference") (OtherBodyIndex :type Integer) (bFromSweep :type Boolean) (SweepResult :type "HitResult Structure (by ref)"))
  (bind (_direction _movement) (`Timeline|Movement` :!label _label)
    (:`Update`
      (`SceneComponent.K2_SetRelativeLocation` (`self.DoorL`) (`KismetMathLibrary.VLerp` (`self.StartPos`) (`self.EndPos`) _movement) false false)
      (`SceneComponent.K2_SetRelativeLocation` (`self.DoorR`) (`KismetMathLibrary.VLerp` (`self.StartPos2`) (`self.EndPos2`) _movement) false false))))

(event `self.Trigger.OnComponentEndOverlap`
  (params (OverlappedComponent :type "PrimitiveComponent Object Reference") (OtherActor :type "Actor Object Reference") (OtherComp :type "PrimitiveComponent Object Reference") (OtherBodyIndex :type Integer))
  (goto _label :!via `Reverse`))

(fn `UserConstructionScript`)
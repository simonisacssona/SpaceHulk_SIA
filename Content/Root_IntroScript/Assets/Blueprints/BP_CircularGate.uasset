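; BP_CircularGate is a gate of four pieces that swings while something overlaps its trigger and returns when the overlap ends.
; Trigger begin overlap plays the Rotate timeline and end overlap reverses it, with no check on the overlapping actor.
; Each timeline update lerps the relative rotation of the four gate components, each turning a quarter turn in yaw from its own offset, forming a pinwheel motion.
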(event `self.Trigger.OnComponentBeginOverlap`
  (params (OverlappedComponent :type "PrimitiveComponent Object Reference") (OtherActor :type "Actor Object Reference") (OtherComp :type "PrimitiveComponent Object Reference") (OtherBodyIndex :type Integer) (bFromSweep :type Boolean) (SweepResult :type "HitResult Structure (by ref)"))
  (bind (_direction _roation_timeline) (`Timeline|Rotate` :!label _label)
    (:`Update`
      (`SceneComponent.K2_SetRelativeRotation` (`self.Gate`) (`KismetMathLibrary.RLerp` (struct) (struct :`Pitch` -90.0) _roation_timeline) false false)
      (`SceneComponent.K2_SetRelativeRotation` (`self.Gate_2`) (`KismetMathLibrary.RLerp` (struct :`Pitch` 90.0) (struct) _roation_timeline) false false)
      (`SceneComponent.K2_SetRelativeRotation` (`self.Gate_3`) (`KismetMathLibrary.RLerp` (struct :`Pitch` 180.0) (struct :`Pitch` 90.0) _roation_timeline) false false)
      (`SceneComponent.K2_SetRelativeRotation` (`self.Gate_4`) (`KismetMathLibrary.RLerp` (struct :`Pitch` -90.0) (struct :`Pitch` -180.0) _roation_timeline) false false))))

(event `self.Trigger.OnComponentEndOverlap`
  (params (OverlappedComponent :type "PrimitiveComponent Object Reference") (OtherActor :type "Actor Object Reference") (OtherComp :type "PrimitiveComponent Object Reference") (OtherBodyIndex :type Integer))
  (goto _label :!via `Reverse`))

(fn `UserConstructionScript`)